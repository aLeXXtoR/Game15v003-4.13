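; Music actor that keeps its MusicAmbient audio volume in sync with the player's saved options.
; OptionChanged loads OptionsSlot, multiplies master and music volume, applies the result and prints it for debugging.
; It runs at BeginPlay and is bound to the Gamw15MainMenu options-changed event.
; The menu lookup and bind repeat every Tick through a gate that starts open and is never closed.
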(event Custom|OptionChanged
  (bind _returnvalue (SaveGame|LoadGamefromSlot "OptionsSlot"))
  (bind _asoptions_menu_save_game (Utilities|Casting|CastToOptionsMenuSaveGame _returnvalue))
  (Audio|Components|Audio|SetVolumeMultiplier (Variables|Default|GetMusicAmbient) (* (Variables|/Game/BluePrints/SaveData/OptionsMenuSaveGame.OptionsMenuSaveGame_C|GetmasterVolume _asoptions_menu_save_game) (Variables|/Game/BluePrints/SaveData/OptionsMenuSaveGame.OptionsMenuSaveGame_C|GetmusicVolume _asoptions_menu_save_game)) :!class /Script/Engine.AudioComponent)
  (Development|PrintString (Utilities|String|Append "Music = " (Utilities|String|ToString(Float) (* (Variables|/Game/BluePrints/SaveData/OptionsMenuSaveGame.OptionsMenuSaveGame_C|GetmasterVolume _asoptions_menu_save_game) (Variables|/Game/BluePrints/SaveData/OptionsMenuSaveGame.OptionsMenuSaveGame_C|GetmusicVolume _asoptions_menu_save_game))))))

(event EventBeginPlay
  (CallFunction|OptionChanged)
  (Utilities|FlowControl|Gate false
    (:Exit
      (bind _foundwidgets (Widget|GetAllWidgetsOfClass "/Game/BluePrints/Interface/Gamw15MainMenu.Gamw15MainMenu_C" true))
      (bind _asgamw_15main_menu (Utilities|Casting|CastToGamw15MainMenu (Utilities|Array|Get(acopy) _foundwidgets)))
      (EventDispatchers|BindEventtoOptionsChangedinMenu _asgamw_15main_menu (delegate Custom|OptionChanged)))))

(event Collision|EventActorBeginOverlap
  (params (OtherActor :type Actor%20Object%20Reference)))

(event EventTick
  (params (DeltaSeconds :type Float%20%28single-precision%29))
  (Utilities|FlowControl|Gate false
    (:Exit
      (bind _foundwidgets (Widget|GetAllWidgetsOfClass "/Game/BluePrints/Interface/Gamw15MainMenu.Gamw15MainMenu_C" true))
      (bind _asgamw_15main_menu (Utilities|Casting|CastToGamw15MainMenu (Utilities|Array|Get(acopy) _foundwidgets)))
      (EventDispatchers|BindEventtoOptionsChangedinMenu _asgamw_15main_menu (delegate Custom|OptionChanged)))))

(fn ConstructionScript)
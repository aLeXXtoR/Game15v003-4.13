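; PB_InfoLeaf is an info display actor that shows the player's current score and time on text render components.
; It caches the Game15PlayerCharacter on BeginPlay, then refreshes both texts from that character every Tick.
; A helper function formats seconds as minutes:seconds with zero-padded seconds, using Round rather than Floor for both parts.
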(event EventBeginPlay
  (bind _asgame_15player_character (Utilities|Casting|CastToGame15PlayerCharacter (Game|GetPlayerCharacter 0)))
  (Variables|Default|SetmyCharacter _asgame_15player_character))

(event Collision|EventActorBeginOverlap
  (params (OtherActor :type Actor%20Object%20Reference)))

(event EventTick
  (params (DeltaSeconds :type Float%20%28single-precision%29))
  (Rendering|Components|TextRender|SetText (Variables|Default|GetTextRenderScore) (Utilities|Text|ToText(Integer) (Variables|/Game/BluePrints/Game15PlayerCharacter.Game15PlayerCharacter_C|GetcurrentScore (Variables|Default|GetmyCharacter))))
  (bind _timeinstring (CallFunction|GetTimefromFloat (Variables|/Game/BluePrints/Game15PlayerCharacter.Game15PlayerCharacter_C|GetcurrentTime (Variables|Default|GetmyCharacter))))
  (Rendering|Components|TextRender|SetText (Variables|Default|GetTextRenderTime) (Utilities|Text|ToText(String) _timeinstring)))

(fn ConstructionScript)

(fn GetTimefromFloat
  (params (timeInSecond :type Float%20%28single-precision%29))
  (bind _returnvalue (Math|Float|%(Float) timeInSecond 6e+01))
  (bind _returnvalue_2 (Math|Float|Round _returnvalue))
  (bind _returnvalue_3 (Utilities|String|ToString(Integer) _returnvalue_2))
  (if (< _returnvalue_2 10)
    (LocalVariables|SetnewString (Utilities|String|Append "0" _returnvalue_3))
    (else
      (LocalVariables|SetnewString _returnvalue_3)))
  (return (Utilities|String|Append (Utilities|String|ToString(Integer) (Math|Float|Round (/ timeInSecond 6e+01))) " : " (LocalVariables|GetnewString))))
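; Numbered wooden tile actor for a 15 puzzle game.
; A click reports the tile's index and movement direction to ChipComponent, while eventMoveChip slides it between two points on a timeline and plays a sound on arrival.
; The construction script picks the digit mesh and builds dynamic material instances with random wood tints and texture offsets, generated once so every LOD matches.
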(event Custom|eventMoveChip
  (params (start :type Vector) (end :type Vector) (masterVolume :type Float%20%28single-precision%29))
  (bind _move (Timeline|Timeline_0 PlayFromStart)
    (:Update
      (Transformation|SetActorLocation (Math|Vector|Lerp(Vector) start end _move) false false))
    (:Finished
      (Audio|PlaySoundatLocation "/Game/Music/bom.bom" (Math|Vector|Lerp(Vector) start end _move) "0, 0, 0" (* masterVolume 0.5)))))

(event Custom|ChangeBlockMovementInt
  (params (MovementInt :type Integer))
  (Variables|Default|SetMoveDirectionInt MovementInt))

(event EventBeginPlay)

(event Collision|EventActorBeginOverlap
  (params (OtherActor :type Actor%20Object%20Reference)))

(event EventTick
  (params (DeltaSeconds :type Float%20%28single-precision%29)))

(event MouseInput|EventActorOnClicked
  (params (ButtonPressed :type Key%20Structure :default "AnyKey"))
  (Class|ChipLogicInterface|ClickChip(Message) (Variables|Default|GetchipComponent) (- (Variables|Default|GetChipNumber) 1) self (Variables|Default|GetMoveDirectionInt)))

(fn ConstructionScript
  (bind _game15_chipvalue (Variables|Default|GetGame15_ChipValue))
  (Components|StaticMesh|SetStaticMesh _game15_chipvalue (Utilities|Array|Get(acopy) (Variables|Default|GetChipDigits) (- (Variables|Default|GetChipNumber) 1)))
  (Transformation|SetRelativeScale3D _game15_chipvalue "2.000000,2.000000,2.000000")
  ;[1 1 1] Set Random values - to use the same through LODs
  (for _index (range 0 3)
    (Utilities|Array|SetArrayElem (Variables|Default|Getcurrent_tint) _index (Math|Conversions|ToVector(LinearColor) (Utilities|RandomTintColor)) true)
    (Utilities|Array|SetArrayElem (Variables|Default|Getcurrent_offset) _index (* (Math|Random|RandomFloat) 0.2) true))
  (for (_array_element _array_index) (Variables|Default|GetLOD_indexes) ; Set Material to each LOD
    (Variables|Default|SetLOD_mat_offset_index _array_element)
    (Variables|Default|SetLOD_index _array_index)
    ;[1 1 1] Tint Material Colors randomly
    (bind _returnvalue (Rendering|Material|CreateDynamicMaterialInstance (Variables|Default|GetGame15_ChipBase) (Variables|Default|GetLOD_mat_offset_index) "/Game/Materials/Wood_A.Wood_A" :!class /Script/Engine.PrimitiveComponent))
    (Rendering|Material|SetVectorParameterValue _returnvalue "WoodTint" (Math|Conversions|ToLinearColor(Vector) (Utilities|Array|Get(acopy) (Variables|Default|Getcurrent_tint))) :!class /Script/Engine.MaterialInstanceDynamic)
    ;[1 1 1] Setting the random Texture offset
    (Rendering|Material|SetScalarParameterValue _returnvalue "TexturePan" (Utilities|Array|Get(acopy) (Variables|Default|Getcurrent_offset)) :!class /Script/Engine.MaterialInstanceDynamic)
    (bind _returnvalue_2 (Rendering|Material|CreateDynamicMaterialInstance (Variables|Default|GetGame15_ChipBase) (+ (Variables|Default|GetLOD_mat_offset_index) 1) "/Game/Materials/Wood_B.Wood_B" :!class /Script/Engine.PrimitiveComponent))
    (Rendering|Material|SetVectorParameterValue _returnvalue_2 "WoodTint" (Math|Conversions|ToLinearColor(Vector) (Utilities|Array|Get(acopy) (Variables|Default|Getcurrent_tint) 1)) :!class /Script/Engine.MaterialInstanceDynamic)
    (Rendering|Material|SetScalarParameterValue _returnvalue_2 "TexturePan" (Utilities|Array|Get(acopy) (Variables|Default|Getcurrent_offset) 1) :!class /Script/Engine.MaterialInstanceDynamic)
    (bind _returnvalue_3 (Rendering|Material|CreateDynamicMaterialInstance (Variables|Default|GetGame15_ChipBase) (+ (Variables|Default|GetLOD_mat_offset_index) 2) "/Game/Materials/Wood_B2.Wood_B2" :!class /Script/Engine.PrimitiveComponent))
    (Rendering|Material|SetVectorParameterValue _returnvalue_3 "WoodTint" (Math|Conversions|ToLinearColor(Vector) (Utilities|Array|Get(acopy) (Variables|Default|Getcurrent_tint) 2)) :!class /Script/Engine.MaterialInstanceDynamic)
    (Rendering|Material|SetScalarParameterValue _returnvalue_3 "TexturePan" (Utilities|Array|Get(acopy) (Variables|Default|Getcurrent_offset) 2) :!class /Script/Engine.MaterialInstanceDynamic)
    ;[1 1 1] Tint Material Colors randomly for Digits
    (bind _returnvalue_4 (Rendering|Material|CreateDynamicMaterialInstance (Variables|Default|GetGame15_ChipValue) (Variables|Default|GetLOD_index) "/Game/Materials/Digits_Mat.Digits_Mat" :!class /Script/Engine.PrimitiveComponent))
    (Rendering|Material|SetVectorParameterValue _returnvalue_4 "WoodTint" (Math|Conversions|ToLinearColor(Vector) (Utilities|Array|Get(acopy) (Variables|Default|Getcurrent_tint) 3)) :!class /Script/Engine.MaterialInstanceDynamic)))
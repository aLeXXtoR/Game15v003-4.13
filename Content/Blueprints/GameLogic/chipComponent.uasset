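; Actor component that handles clicks on chips in a sliding "15" puzzle.
; On a click with a valid direction before the win, it raises the player's score, tells LevelLogic to recalculate the grid, and triggers the chip's move event.
; The move offset comes from a direction-vector lookup, and the first scored move switches on the player's GamePlay flag through a DoOnce.
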(event EventBeginPlay
  (bind _outactors (Actor|GetAllActorsOfClass "/Game/Blueprints/GameLogic/levelLogic.levelLogic_C"))
  (Variables|Default|SetgameLogic (Utilities|Array|Get(acopy) _outactors))
  (bind _asgame_15player_character (Utilities|Casting|CastToGame15PlayerCharacter (Game|GetPlayerCharacter 0)))
  (Variables|Default|SetmyCharacter _asgame_15player_character))

(event EventTick
  (params (DeltaSeconds :type Float%20%28single-precision%29)))

(event EventClickChip
  (params (blockId :type Integer) (blockActor :type Game%20Chip%20Object%20Reference) (moveDirectionInt :type Integer))
  ;[1 1 1] click
  (Variables|Default|SetblockId blockId)
  (bind _output_get (Variables|Default|SetblockActor blockActor))
  (Variables|Default|SetmoveDirectionInt moveDirectionInt)
  (if (and (!= (Variables|Default|GetmoveDirectionInt) 0) (not (Variables|/Game/BluePrints/Game15PlayerCharacter.Game15PlayerCharacter_C|GetWinFlag (Variables|Default|GetmyCharacter))))
    (CallFunction|AddScore)
    (bind _output_get_2 (Variables|Default|SetmyLocation (Transformation|GetActorLocation _output_get)))
    (bind _output_get_3 (Variables|Default|SetmovingOffset (Utilities|Array|Get(acopy) (Variables|Default|GetmoveDirectionVector) (Variables|Default|GetmoveDirectionInt))))
    (Default|RecalculateGridMovement (Variables|Default|GetgameLogic) (Variables|Default|GetblockId))
    (Default|EventMoveChip (Variables|Default|GetblockActor) _output_get_2 (+ _output_get_2 _output_get_3) 1.0)))

(fn AddScore
  (bind _mycharacter (Variables|Default|GetmyCharacter))
  (Variables|/Game/BluePrints/Game15PlayerCharacter.Game15PlayerCharacter_C|SetcurrentScore _mycharacter (+ (Variables|/Game/BluePrints/Game15PlayerCharacter.Game15PlayerCharacter_C|GetcurrentScore _mycharacter) 1))
  (Utilities|FlowControl|DoOnce false
    (:Completed
      (Variables|/Game/BluePrints/Game15PlayerCharacter.Game15PlayerCharacter_C|SetgamePlay (Variables|Default|GetmyCharacter) true))))
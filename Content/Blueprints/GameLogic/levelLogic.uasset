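; Level logic for a 15-puzzle game that creates the HUD, shuffles GameChip actors and counts play time.
; It sorts chips by number, rerandomizes until an inversion-parity check passes, then animates the shuffle with lift, swap and lower timelines.
; RecalculateGridMovement updates the 4x4 board after a move and gives chips beside the blank their slide direction.
; CheckWin's win branch is hard-wired false and SaveStat is empty.
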(event Custom|StartShuffle3
  (bind _down (Timeline|TimelineLiftDown PlayFromStart)
    (:Update
      (Shuffle|ShuffleDown _down))))

(event Custom|StartShuffle2
  (bind _swap (Timeline|TimelineSwapBlock PlayFromStart)
    (:Update
      (Shuffle|ShuffleBlock _swap)
      (Shuffle|ShuffleRotateDown _swap))
    (:Finished
      (CallFunction|StartShuffle3))))

(event Custom|OptionChanged)

(event Custom|StartShuffle
  (bind _up (Timeline|TimelineLiftUp PlayFromStart)
    (:Update
      (Shuffle|ShuffleUp _up)
      (Shuffle|ShuffleRotateUp _up))))

(event EventBeginPlay
  ;[1 1 1] Begin Play
  (bind _returnvalue (UserInterface|CreateWidget "/Game/BluePrints/Interface/Game15HUD.Game15HUD_C"))
  (UserInterface|Viewport|AddtoViewport _returnvalue 0)
  (bind _asgame_15player_character (Utilities|Casting|CastToGame15PlayerCharacter (Game|GetPlayerCharacter 0)))
  (Variables|Default|SetmyCharacter _asgame_15player_character)
  (Utilities|FlowControl|Delay 0.5)
  (Grid|CreateArrayBlockActor))

(event EventTick
  (params (DeltaSeconds :type Float%20%28single-precision%29))
  ;[1 1 1] Event Tick
  (if (Variables|/Game/BluePrints/Game15PlayerCharacter.Game15PlayerCharacter_C|GetgamePlay (Variables|Default|GetmyCharacter))
    (Utilities|FlowControl|Delay 1.0)
    (Variables|/Game/BluePrints/Game15PlayerCharacter.Game15PlayerCharacter_C|SetcurrentTime (Variables|Default|GetmyCharacter) (+ 1.0 (Variables|/Game/BluePrints/Game15PlayerCharacter.Game15PlayerCharacter_C|GetcurrentTime (Variables|Default|GetmyCharacter))))))

(event Collision|EventActorBeginOverlap
  (params (OtherActor :type Actor%20Object%20Reference)))

(fn ConstructionScript)

(fn CreateArrayBlockActor
  (bind _returnvalue (Math|Vector|MakeVector 0.0 0.0 25.0))
  (bind _randomblockposition (Variables|Grid|GetRandomBlockPosition))
  (bind _outactors (Actor|GetAllActorsOfClass "/Game/Blueprints/Model/GameChip.GameChip_C"))
  (bind _arrayout (Grid|SortArrayOfChips _outactors))
  (Variables|Grid|SetinitalArrayBlockActor _arrayout)
  (Utilities|FlowControl|Sequence
    (:then_0
      (Grid|CreateBlockInitalLocation)
      (CallFunction|StartShuffle))
    (:then_1
      ;[1 1 1] Create integer array and check on solution
      (while (Variables|Grid|GetarrayNeedRecreate)
        (Grid|RandomizeArray)
        (gameStatus|CheckSolution))
      ;[1 1 1] Create Actor Block Array
      (for _array_element _randomblockposition
        (Utilities|Array|Add (Variables|Default|GetarrayBlockActor) (Utilities|Array|Get(acopy) (Variables|Grid|GetinitalArrayBlockActor) (- _array_element 1))))
      (Variables|Grid|SetcurrentBlockPosition _randomblockposition)
      (Utilities|Array|Add (Variables|Grid|GetcurrentBlockPosition) 0)
      ;[1 1 1] UpBlockLocation
      (for _index (range 0 14)
        (Utilities|Array|Add (Variables|Shuffle|GetinitalUpBlockLocation) (+ (Transformation|GetActorLocation (Utilities|Array|Get(acopy) (Variables|Grid|GetinitalArrayBlockActor) _index)) _returnvalue))
        (Utilities|Array|Add (Variables|Shuffle|GetUpBlockLocation) (+ (Transformation|GetActorLocation (Utilities|Array|Get(acopy) (Variables|Default|GetarrayBlockActor) _index)) _returnvalue)))
      (CallFunction|StartShuffle2)
      (bind _asgame_chip (Utilities|Casting|CastToGameChip (Utilities|Array|Get(acopy) (Variables|Default|GetarrayBlockActor) 11)))
      (Default|ChangeBlockMovementInt _asgame_chip 4)
      (bind _asgame_chip_2 (Utilities|Casting|CastToGameChip (Utilities|Array|Get(acopy) (Variables|Default|GetarrayBlockActor) 14)))
      (Default|ChangeBlockMovementInt _asgame_chip_2 3))))

(fn RecalculateGridMovement
  (params (blockIdClicked :type Integer))
  (bind _currentblockposition (Variables|Grid|GetcurrentBlockPosition))
  (bind _currentblockposition_2 (Variables|Grid|GetcurrentBlockPosition))
  (Variables|Grid|SetnewBlockBlankPosition (Variables|Grid|GetblockBlankPosition))
  (Variables|Grid|SetblockIdClicked blockIdClicked)
  (for _index (range 0 14) ; цикл по массиву движений
    (Utilities|Array|SetArrayElem (Variables|Grid|GetcurrentBlockDirection) _index 0) ; Обнуляем все движения
  )
  (Utilities|Array|SetArrayElem _currentblockposition (Utilities|Array|FindItem _currentblockposition (+ (Variables|Grid|GetblockIdClicked) 1)) 0)
  (Utilities|Array|SetArrayElem _currentblockposition_2 (Variables|Grid|GetnewBlockBlankPosition) (+ (Variables|Grid|GetblockIdClicked) 1))
  (Variables|Grid|SetblockBlankPosition (Utilities|Array|FindItem _currentblockposition_2 0))
  (Variables|Grid|SetblankX (/ (Variables|Grid|GetblockBlankPosition) 4))
  (Variables|Grid|SetblankY (Math|Integer|%(Integer) (Variables|Grid|GetblockBlankPosition) 4))
  (Utilities|FlowControl|Sequence
    (:then_0
      (Grid|GetLeftby0))
    (:then_1
      (Grid|GetRightby0))
    (:then_2
      (Grid|GetTopby0))
    (:then_3
      (Grid|GetBottomby0))
    (:then_4
      (for (_array_element _array_index) (Variables|Grid|GetcurrentBlockDirection)
        (bind _asgame_chip (Utilities|Casting|CastToGameChip (Utilities|Array|Get(acopy) (Variables|Default|GetarrayBlockActor) (Utilities|Array|FindItem (Variables|Grid|GetRandomBlockPosition) (+ _array_index 1)))))
        (Default|ChangeBlockMovementInt _asgame_chip _array_element))
      (gameStatus|CheckWin))))

(fn GetLeftby0
  (if (>= (- (Variables|Grid|GetblankY) 1) 0)
    (Utilities|Array|SetArrayElem (Variables|Grid|GetcurrentBlockDirection) (- (Utilities|Array|Get(acopy) (Variables|Grid|GetcurrentBlockPosition) (- (+ (* (Variables|Grid|GetblankX) 4) (Variables|Grid|GetblankY)) 1)) 1) 3)))

(fn GetRightby0
  (if (<= (+ (Variables|Grid|GetblankY) 1) 3)
    (Utilities|Array|SetArrayElem (Variables|Grid|GetcurrentBlockDirection) (- (Utilities|Array|Get(acopy) (Variables|Grid|GetcurrentBlockPosition) (+ (+ (* (Variables|Grid|GetblankX) 4) (Variables|Grid|GetblankY)) 1)) 1) 1)))

(fn GetTopby0
  (if (>= (- (Variables|Grid|GetblankX) 1) 0)
    (Utilities|Array|SetArrayElem (Variables|Grid|GetcurrentBlockDirection) (- (Utilities|Array|Get(acopy) (Variables|Grid|GetcurrentBlockPosition) (+ (* (- (Variables|Grid|GetblankX) 1) 4) (Variables|Grid|GetblankY))) 1) 4)))

(fn GetBottomby0
  (if (<= (+ (Variables|Grid|GetblankX) 1) 3)
    (Utilities|Array|SetArrayElem (Variables|Grid|GetcurrentBlockDirection) (- (Utilities|Array|Get(acopy) (Variables|Grid|GetcurrentBlockPosition) (+ (* (+ (Variables|Grid|GetblankX) 1) 4) (Variables|Grid|GetblankY))) 1) 2)))

(fn RandomizeArray
  (for _index (range 0 14)
    (bind _output_get (LocalVariables|SetI _index))
    (bind _output_get_2 (LocalVariables|SetJ (Math|Random|RandomIntegerinRange 0 _index)))
    (LocalVariables|SetswapValue (Utilities|Array|Get(acopy) (Variables|Grid|GetRandomBlockPosition) _output_get))
    (Utilities|Array|SetArrayElem (Variables|Grid|GetRandomBlockPosition) (LocalVariables|GetI) (Utilities|Array|Get(acopy) (Variables|Grid|GetRandomBlockPosition) _output_get_2)) ; I=J
    (Utilities|Array|SetArrayElem (Variables|Grid|GetRandomBlockPosition) (LocalVariables|GetJ) (LocalVariables|GetswapValue)) ; J=swp
  ))

(fn CheckSolution
  ;[1 1 1] Проверка на решаемость
  (LocalVariables|Setcount 0)
  (LocalVariables|SetcheckBlockPosition (Variables|Grid|GetRandomBlockPosition))
  (Utilities|Array|Add (LocalVariables|GetcheckBlockPosition) 0)
  (for (_array_element _array_index) (LocalVariables|GetcheckBlockPosition)
    (if (> _array_element 0)
      (for _index (range 0 _array_index)
        (if (> (Utilities|Array|Get(acopy) (LocalVariables|GetcheckBlockPosition) _index) _array_element)
          (LocalVariables|Setcount (+ 1 (LocalVariables|Getcount)))))))
  (LocalVariables|Setcount (+ (LocalVariables|Getcount) (+ (/ (Utilities|Array|FindItem (LocalVariables|GetcheckBlockPosition) 0) 4) 1)))
  (if (<= (Math|Integer|%(Integer) (LocalVariables|Getcount) 2) 0)
    (Variables|Grid|SetarrayNeedRecreate false)))

(fn CheckWin
  (bind _mycharacter (Variables|Default|GetmyCharacter))
  ;[1 1 1] check win
  (bind (_array_element _array_index) (Utilities|Array|ForEachLoopwithBreak (Variables|Grid|GetcurrentBlockPosition))
    (:LoopBody
      (if (== (Utilities|Array|Get(acopy) (Variables|GameStatus|GetpositionBlockWin) _array_index) _array_element)
        _))
    (:Completed
      (if false
        (Audio|PlaySoundatLocation "/Game/Music/zombieWin.zombieWin" (Transformation|GetActorLocation (Variables|Default|GetmyCharacter)) "0, 0, 0" (Variables|Options|GetVolumeEffect))
        (Variables|/Game/BluePrints/Game15PlayerCharacter.Game15PlayerCharacter_C|SetWinFlag _mycharacter false)
        (Variables|/Game/BluePrints/Game15PlayerCharacter.Game15PlayerCharacter_C|SetgamePlay _mycharacter false)
        (Options|SaveStat)))))

(fn ShuffleUp
  (params (alpha :type Float%20%28single-precision%29))
  (for (_array_element _array_index) (Variables|Grid|GetinitalArrayBlockActor)
    (Transformation|SetActorLocation _array_element (Math|Vector|Lerp(Vector) (Utilities|Array|Get(acopy) (Variables|Shuffle|GetinitalBlockLocation) _array_index) (+ (Utilities|Array|Get(acopy) (Variables|Shuffle|GetinitalBlockLocation) _array_index) "0, 0,25.000000") alpha) false false)))

(fn CreateBlockInitalLocation
  ;[1 1 1] initalBlockLocation
  (for _array_element (Variables|Grid|GetinitalArrayBlockActor)
    (Utilities|Array|Add (Variables|Shuffle|GetinitalBlockLocation) (Transformation|GetActorLocation _array_element))))

(fn ShuffleRotateUp
  (params (alpha :type Float%20%28single-precision%29))
  (for _array_element (Variables|Grid|GetinitalArrayBlockActor)
    (Transformation|SetActorRelativeRotation _array_element (Math|Rotator|Lerp(Rotator) "0,90.000000, 0" "180.000000,90.000000,360.000000" alpha))))

(fn ShuffleBlock
  (params (alpha :type Float%20%28single-precision%29))
  (for (_array_element _array_index) (Variables|Default|GetarrayBlockActor)
    (Transformation|SetActorLocation _array_element (Math|Vector|Lerp(Vector) (Utilities|Array|Get(acopy) (Variables|Shuffle|GetUpBlockLocation) _array_index) (Utilities|Array|Get(acopy) (Variables|Shuffle|GetinitalUpBlockLocation) _array_index) alpha) false true)))

(fn ShuffleRotateDown
  (params (alpha :type Float%20%28single-precision%29))
  (for _array_element (Variables|Grid|GetinitalArrayBlockActor)
    (Transformation|SetActorRelativeRotation _array_element (Math|Rotator|Lerp(Rotator) "360.000000,0.000000,180.000000" "0.000000,0.000000,0.000000" alpha))))

(fn ShuffleDown
  (params (alpha :type Float%20%28single-precision%29))
  (for (_array_element _array_index) (Variables|Default|GetarrayBlockActor)
    (Transformation|SetActorLocation _array_element (Math|Vector|Lerp(Vector) (Utilities|Array|Get(acopy) (Variables|Shuffle|GetinitalUpBlockLocation) _array_index) (Utilities|Array|Get(acopy) (Variables|Shuffle|GetinitalBlockLocation) _array_index) alpha) false false)))

(fn SaveStat)

(fn SortArrayOfChips
  (params (arrayIn :type Array%20of%20Game%20Chip%20Object%20References))
  (bind _array (LocalVariables|Getarray))
  (for _index (range 1 15)
    (bind _array_element (Utilities|Array|ForEachLoopwithBreak arrayIn :!label _label)
      (:LoopBody
        (bind _asgame_chip (Utilities|Casting|CastToGameChip _array_element))
        (if (== _index (Variables|/Game/Blueprints/Model/GameChip.GameChip_C|GetChipNumber _asgame_chip))
          (Utilities|Array|Add _array _array_element)
          (goto _label Break)))))
  (return _array))